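; Procedural level actor for what appears to be a brick-breaker game, also managing bonus drops.
; Construction script tiles floor and walls from an enum-keyed struct map, tags one wall as KillZ, then adds a player start and tapering block rows as child actors.
; BeginPlay derives camera and light positions from averaged tile locations.
; Bonus spawning is gated by active-bonus flags, with random red or blue material and delegate bindings.
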(event `self.ReceiveBeginPlay`
  (bind (_returnvalue _returnvalue2 _returnvalue3 _returnvalue4) (`self.CamLocationCalc`))
  (bind (_returnvalue_2 _returnvalue2_2 _returnvalue3_2 _returnvalue4_2) (`self.CamLocationCalc`))
  (`|ExecutionSequence`
    (:`then_0`
      (message `/Game/Blueprints/Interfaces/BPI_Cam.CamLocation` _returnvalue (`KismetMathLibrary.MakeVector` _returnvalue2 _returnvalue3 _returnvalue4)))
    (:`then_1`
      (`SceneComponent.K2_SetWorldLocation` (`self.DirectionalLight`) (`KismetMathLibrary.MakeVector` _returnvalue2_2 _returnvalue3_2 _returnvalue4_2) false false))))

(event `/Game/Blueprints/Interfaces/BPI_Bonus.SpawnBonus`
  (params (Location :type "Vector Structure"))
  (`self.Bonus` Location))

(event `/Game/Blueprints/Interfaces/BPI_Bonus.BonusEnds`
  (set `self.HasBonus` false))

(event `/Game/Blueprints/Interfaces/BPI_Bonus.BonusBallSlowDown`
  (params (HasBonus :type Boolean))
  (bind _output_get (set `self.BallHasBonus` HasBonus))
  (if (not _output_get)
    (`/Game/Blueprints/Interfaces/BPI_Bonus.BonusEnds`)))

(event `/Game/Blueprints/Interfaces/BPI_Bonus.ApplyingBonus`
  (set `self.HasBonus` true))

(event `/Game/Blueprints/Interfaces/BPI_Bonus.BonusOnTarget`
  (params (HasBonus :type Boolean))
  (bind _output_get (set `self.BallHasBonus` HasBonus))
  (if (not _output_get)
    (`/Game/Blueprints/Interfaces/BPI_Bonus.BonusEnds`)))

(fn `AddStructs`
  (locals (CubeHeight :type "Float (double-precision)" :default 0.0) (CubeLength :type "Float (double-precision)" :default 0.0) (Cube :type "StaticMesh Object Reference" :default "/Script/Engine.StaticMesh'/Engine/EditorMeshes/AssetViewer/Floor_Mesh.Floor_Mesh'"))
  (bind _cubelength (`local.CubeLength`))
  (bind _cubelength_2 (`local.CubeLength`))
  (bind _cubelength_3 (`local.CubeLength`))
  (bind _cubelength_4 (`local.CubeLength`))
  (bind _returnvalue (`StaticMesh.GetBounds` (`local.Cube`)))
  (bind _returnvalue_2 (* (`local.CubeLength`) 2.0))
  (bind _returnvalue_3 (* (`local.CubeLength`) 2.0))
  (bind _returnvalue_4 (* (`local.CubeLength`) 2.0))
  (bind _returnvalue_5 (* (`local.CubeLength`) 2.0))
  (bind _returnvalue_6 (* (`local.CubeLength`) 2.0))
  (set `local.CubeLength` (.x (`.BoxExtent` (`KismetMathLibrary.BreakBoxSphereBounds` _returnvalue))))
  (set `local.CubeHeight` (.z (`.BoxExtent` (`KismetMathLibrary.BreakBoxSphereBounds` _returnvalue))))
  (`BlueprintMapLibrary.Map_Add` (`self.ObjectsStruct`) "NewEnumerator1" (make `/Game/Blueprints/Structs/S_LevelObjects` _returnvalue_2 _returnvalue_2))
  (`BlueprintMapLibrary.Map_Add` (`self.ObjectsStruct`) "NewEnumerator2" (make `/Game/Blueprints/Structs/S_LevelObjects` _returnvalue_4 _returnvalue_4 _cubelength_2 (struct :`Roll` 90.0) 0.0 (+ _cubelength_2 (* (`local.CubeHeight`) 2.0))))
  (`BlueprintMapLibrary.Map_Add` (`self.ObjectsStruct`) "NewEnumerator3" (make `/Game/Blueprints/Structs/S_LevelObjects` _returnvalue_5 _returnvalue_5 _cubelength_3 (struct :`Pitch` -90.0) (+ _cubelength_3 (* (`local.CubeHeight`) 2.0))))
  (`BlueprintMapLibrary.Map_Add` (`self.ObjectsStruct`) "NewEnumerator4" (make `/Game/Blueprints/Structs/S_LevelObjects` _returnvalue_6 _returnvalue_6 _cubelength_4 (struct :`Roll` -90.0) 0.0 (+ (* _cubelength_4 -1.0) (* (`local.CubeHeight`) -2.0))))
  (`BlueprintMapLibrary.Map_Add` (`self.ObjectsStruct`) "NewEnumerator5" (make `/Game/Blueprints/Structs/S_LevelObjects` _returnvalue_3 _returnvalue_3 _cubelength (struct :`Pitch` 90.0) (+ (* _cubelength -1.0) (* (`local.CubeHeight`) -2.0)) 0.0 "KillZ"))
  (return))

(fn `Apply Bonus`
  (bind _blocklocations (`self.BlockLocations`))
  (bind _output (`|GetArrayItem` _blocklocations (/ (`self.SideY`) 2)))
  (bind _output_2 (`|GetArrayItem` _blocklocations (- (`KismetArrayLibrary.Array_Length` _blocklocations) 1)))
  (bind (_outhit _returnvalue) (`KismetSystemLibrary.BoxTraceSingle` _output _output_2 (`KismetMathLibrary.MakeVector` (.x _output) (.y _output_2) 50.0) (struct) "TraceTypeQuery1"))
  (if _returnvalue
    (if (`self.ActorHasTag` (`.HitActor` (`GameplayStatics.BreakHitResult` _outhit)) "Block")
      (set `self.HasBonus` true))))

(fn `BlockConstruction`
  (params (BlocksMaxLength :type "Float (double-precision)") (Location :type "Vector Structure"))
  (locals (Y_0 :type Integer) (Y :type Integer :default 5) (X :type Integer :default 5) (Padding :type Integer :default 330) (CubeScaleY :type "Float (double-precision)" :default 1.0))
  (set `local.Y_0` 0)
  (bind _output_get (set `local.Y` (/ BlocksMaxLength (`local.Padding`))))
  (set `self.SideY` _output_get)
  (bind _output_get_2 (set `local.X` (/ _output_get 2)))
  (set `self.SideX` _output_get_2)
  (for _index (range (+ (`local.X`) 1))
    (for _index_2 (range (`local.Y_0`) (+ (`local.Y`) 1))
      (bind _returnvalue (`AddComponent|NODE_AddChildActorComponent-1` :`RelativeTransform` (`KismetMathLibrary.MakeTransform` (+ Location (`KismetMathLibrary.MakeVector` (`KismetMathLibrary.Conv_IntToDouble` (* _index (`local.Padding`) (`self.CubeScaleX`))) (`KismetMathLibrary.Conv_IntToDouble` (* _index_2 (`local.Padding`) (`local.CubeScaleY`))))) (struct) (`KismetMathLibrary.MakeVector` (`self.CubeScaleX`) (`local.CubeScaleY`) 0.2))))
      (`KismetArrayLibrary.Array_Add` (`self.BlockLocations`) (`SceneComponent.K2_GetComponentLocation` _returnvalue)))
    (set `local.Y_0` (+ (`local.Y_0`) 1))
    (set `local.Y` (- (`local.Y`) 1))))

(fn `Blocks Length and Location Calc`
  (returns (BlocksLength :type "Float (double-precision)") (FirstBlockLocation :type "Vector Structure"))
  (bind _value (`BlueprintMapLibrary.Map_Find` (`self.ObjectsStruct`) "NewEnumerator4"))
  (bind (_output_x _output_y _output_z) (`KismetMathLibrary.BreakVector` (`|GetArrayItem` (`self.ConstructLocations`))))
  (bind (_output_x_2 _output_y_2) (`KismetMathLibrary.BreakVector` (`|GetArrayItem` (`self.ConstructLocations`) (- (`self.SideY`) 1))))
  (bind _returnvalue (/ (`.YOffset_15_13CEE37A420C6ACB3FE066BAF1479D75` (break `/Game/Blueprints/Structs/S_LevelObjects` _value)) -6.0))
  (bind _returnvalue_2 (+ _output_y _returnvalue))
  (return (- (- _output_y_2 _returnvalue) _returnvalue_2) (`KismetMathLibrary.MakeVector` (+ _output_x (/ (break `/Game/Blueprints/Structs/S_LevelObjects` _value) 6.0)) _returnvalue_2 (+ _output_z (/ (`.ZOffset_17_E41A7E3444C4090FAED6778A4708231A` (break `/Game/Blueprints/Structs/S_LevelObjects` _value)) 6.0)))))

(fn `Bonus`
  (params (Location :type "Vector Structure"))
  (if (or (`self.CanSpawn`) (and (not (`self.HasBonus`)) (not (`self.BallHasBonus`))))
    (set `self.CanSpawn` false)
    (bind _returnvalue (`|SpawnActorFromClass` "/Game/Blueprints/Bonuses/BP_Bonus.BP_Bonus_C" (`KismetMathLibrary.MakeTransform` Location (struct) (0.25 0.25 0.25)) "AlwaysSpawn" "MultiplyWithRoot" null null))
    (add `/Game/Blueprints/Bonuses/BP_Bonus.DeathOnZ` _returnvalue (`|CreateDelegate` :!event `BonusKilledOnZFunc`))
    (add `/Game/Blueprints/Bonuses/BP_Bonus.DeathOnPawn` _returnvalue (`|CreateDelegate` :!event `Apply Bonus`))
    (add `/Game/Blueprints/Bonuses/BP_Bonus.BlockImmortal` _returnvalue (`|CreateDelegate` :!event `BonusBlockImmortal`))
    (add `/Game/Blueprints/Bonuses/BP_Bonus.PawnSpeedDown` _returnvalue (`|CreateDelegate` :!event `ApplyingBonus`))
    (if (`KismetMathLibrary.RandomBool`)
      (bind _sphere (`/Game/Blueprints/BP_Ball.Sphere` _returnvalue))
      (`PrimitiveComponent.SetMaterial` _sphere 0 "/Game/Materials/MI_BonusBlue.MI_BonusBlue")
      (else
        (`PrimitiveComponent.SetMaterial` _sphere 0 "/Game/Materials/MI_BonusRed.MI_BonusRed")))))

(fn `BonusBlockImmortal`
  (bind _outactors (`GameplayStatics.GetAllActorsOfClassWithTag` "/Game/Blueprints/BP_Block.BP_Block_C" "Block"))
  (for _array_element _outactors
    (`/Game/Blueprints/Interfaces/BPI_Bonus.BonusBlocksImmortal` _array_element)))

(fn `BonusKilledOnZFunc`
  (set `self.CanSpawn` true))

(fn `CamLocationCalc`
  (returns (ReturnValue :type "Pawn Object Reference") (ReturnValue2 :type "Float (double-precision)") (ReturnValue3 :type "Float (double-precision)") (ReturnValue4 :type "Float (double-precision)"))
  (bind _returnvalue (`KismetMathLibrary.GetVectorArrayAverage` (`self.ConstructLocations`)))
  (bind _value (`BlueprintMapLibrary.Map_Find` (`self.ObjectsStruct`) "NewEnumerator5"))
  (bind _returnvalue_2 (/ (`.ZOffset_17_E41A7E3444C4090FAED6778A4708231A` (break `/Game/Blueprints/Structs/S_LevelObjects` _value)) 6.0))
  (bind _returnvalue_3 (/ (break `/Game/Blueprints/Structs/S_LevelObjects` _value) 2.0))
  (return (`GameplayStatics.GetPlayerPawn` 0) (+ (- (.x _returnvalue) _returnvalue_3) (/ _returnvalue_2 3.0)) (- (- (.y _returnvalue) _returnvalue_3) _returnvalue_2) (`KismetMathLibrary.VSizeXY` _returnvalue)))

(fn `ObjectType`
  (params (indX :type Integer) (indY :type Integer))
  (returns (Object :type "/Game/Blueprints/Enums/E_LevelObjects Enum"))
  (locals (X :type Integer) (Y :type Integer))
  (set `local.X` indX)
  (set `local.Y` indY)
  (if (not (or (and (== (`local.X`) 0) (== (`local.Y`) 0)) (and (== (`local.X`) 0) (== (`local.Y`) (`self.LevelY`))) (and (== (`local.X`) (`self.LevelX`)) (== (`local.Y`) 0)) (and (== (`local.X`) (`self.LevelX`)) (== (`local.Y`) (`self.LevelY`)))))
    (if (== (`local.X`) 0)
      (return "NewEnumerator3")
      (elif (== (`local.X`) (`self.LevelX`))
        (return "NewEnumerator5")
        (elif (== (`local.Y`) 0)
          (return "NewEnumerator2")
          (elif (== (`local.Y`) (`self.LevelY`))
            (return "NewEnumerator4")
            (else
              (return "NewEnumerator1"))))))
    (else
      (return "NewEnumerator6"))))

(fn `ProceduralWallsAndFloor`
  (params (SideX :type Integer) (SideY :type Integer))
  (locals (IndexX :type Integer) (IndexY :type Integer) (NewLocalVar :type Integer) (NewLocalVar_0 :type Integer))
  (bind _constructlocations (`self.ConstructLocations`))
  (bind _object (`self.ObjectType` (`local.IndexX`) (`local.IndexY`)))
  (bind (_xoffset _yoffset _zoffset _rotation _locationxdelta _locationydelta _iskillz) (break `/Game/Blueprints/Structs/S_LevelObjects` (`BlueprintMapLibrary.Map_Find` (`self.ObjectsStruct`) _object)))
  (bind _returnvalue (`KismetMathLibrary.MakeVector` (+ (* (`local.IndexX`) _xoffset) _locationxdelta) (+ (* (`local.IndexY`) _yoffset) _locationydelta) _zoffset))
  (bind _result (`/Engine/EditorBlueprintResources/StandardMacros.IncrementInt` SideX)
    (:`  `
      (set `self.LevelX` _result)
      (bind _result_2 (`/Engine/EditorBlueprintResources/StandardMacros.IncrementInt` SideY)
        (:`  `
          (set `self.LevelY` _result_2)
          (for _index (range (+ (`self.LevelX`) 1))
            (set `local.IndexX` _index)
            (for _index_2 (range (+ (`self.LevelY`) 1))
              (set `local.IndexY` _index_2)
              (if (not (`|EnumEquality` _object "NewEnumerator6"))
                (bind _returnvalue_2 (`AddComponent|NODE_AddStaticMeshComponent-0` :`RelativeTransform` (`KismetMathLibrary.MakeTransform` _returnvalue _rotation)))
                (bind _componenttags (`ActorComponent.ComponentTags` _returnvalue_2))
                (bind _returnvalue_3 (`KismetArrayLibrary.Array_Add` _componenttags _iskillz))
                (bind _returnvalue_4 (`KismetArrayLibrary.Array_Add` _constructlocations _returnvalue))
                (if (== (`|GetArrayItem` _componenttags _returnvalue_3) "KillZ")
                  (bind (_output_x _output_y _output_z) (`KismetMathLibrary.BreakVector` (`|GetArrayItem` _constructlocations _returnvalue_4)))
                  (bind _returnvalue_5 (`AddComponent|NODE_AddStaticMeshComponent-9` :`RelativeTransform` (`KismetMathLibrary.MakeTransform` (`KismetMathLibrary.MakeVector` (/ (+ (+ _output_x (/ (`.LocationXDelta_25_9638A0F64FC4DD5089E44FA5E0F03BDC` (break `/Game/Blueprints/Structs/S_LevelObjects` (`BlueprintMapLibrary.Map_Find` (`self.ObjectsStruct`) "NewEnumerator5"))) 2.0)) _output_x) 2.0) _output_y _output_z) (struct :`Pitch` 90.0) (10.0 10.0 10.0))))
                  (`KismetArrayLibrary.Array_Add` (`ActorComponent.ComponentTags` _returnvalue_5) _iskillz))))))))))

(fn `Spawn Player Start`
  (bind _constructlocations (`self.ConstructLocations`))
  (bind _returnvalue (`KismetArrayLibrary.Array_Length` _constructlocations))
  (bind _returnvalue_2 (/ (`.LocationXDelta_25_9638A0F64FC4DD5089E44FA5E0F03BDC` (break `/Game/Blueprints/Structs/S_LevelObjects` (`BlueprintMapLibrary.Map_Find` (`self.ObjectsStruct`) "NewEnumerator5"))) 2.5))
  (bind (_returnvalue_x _returnvalue_y _returnvalue_z) (`KismetMathLibrary.BreakVector` (/ (+ (`|GetArrayItem` _constructlocations (- _returnvalue 1)) (`|GetArrayItem` _constructlocations (- _returnvalue (`self.SideY`) 0))) 2)))
  (`AddComponent|NODE_AddChildActorComponent-9` :`RelativeTransform` (`KismetMathLibrary.MakeTransform` (`KismetMathLibrary.MakeVector` (+ _returnvalue_x _returnvalue_2) _returnvalue_y (- _returnvalue_z (/ _returnvalue_2 3.0))) (struct :`Yaw` 180.0))))

(fn `UserConstructionScript`
  (locals (IndexX :type Integer) (IndexY :type Integer) (BlockMaxLength :type "Float (double-precision)"))
  (bind (_blockslength _firstblocklocation) (`self.Blocks Length and Location Calc`))
  (`|ExecutionSequence`
    (:`then_0`
      (`self.AddStructs`)
      (set `self.SideX` (/ (* (`self.SideY`) 3) 4))
      (`self.ProceduralWallsAndFloor` (`self.SideX`) (`self.SideY`)))
    (:`then_1`
      (`self.Spawn Player Start`))
    (:`then_2`
      (`self.BlockConstruction` _blockslength _firstblocklocation))))
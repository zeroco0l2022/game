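; BP_Bonus is a projectile pickup that launches along X at a random speed and gives a random effect on hitting a Pawn.
; The effect is either an interface message to the pawn (second ball, slow-down, targeting) or a dispatcher call (immortal blocks, pawn speed).
; The rocket case is unreachable because RandomInteger(6) stops at 5.
; It fires a death dispatcher on either pawn or KillZ hits, then destroys itself.
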(event `self.ReceiveBeginPlay`
  ;[0.9267 0.3421 1] BeginPlay
  (`self.InitialSpeed`))

(event `self.ReceiveHit`
  (params (MyComp :type "PrimitiveComponent Object Reference") (Other :type "Actor Object Reference") (OtherComp :type "PrimitiveComponent Object Reference") (bSelfMoved :type Boolean) (HitLocation :type "Vector Structure") (HitNormal :type "Vector Structure") (NormalImpulse :type "Vector Structure") (Hit :type "HitResult Structure (by ref)"))
  (if (`ActorComponent.ComponentHasTag` OtherComp "KillZ")
    (`self.DeathOnZ`)
    (`self.K2_DestroyActor`)
    (elif (`self.ActorHasTag` Other "Pawn")
      (`self.Bonus` Other)
      (`self.DeathOnPawn`))))

(event `Bonus`
  (params (OtherActor :type "Actor Object Reference"))
  (switch `int` (`KismetMathLibrary.RandomInteger` 6)
    (:`0`
      (message `/Game/Blueprints/Interfaces/BPI_Bonus.BonusSecondBall` OtherActor))
    (:`1`
      (message `/Game/Blueprints/Interfaces/BPI_Bonus.BonusBallSlowDown` OtherActor false))
    (:`2`
      (`self.BlockImmortal`))
    (:`3`
      (message `/Game/Blueprints/Interfaces/BPI_Bonus.BonusPawnSpeedDown` OtherActor))
    (:`4`
      (`self.PawnSpeedDown`))
    (:`5`
      (message `/Game/Blueprints/Interfaces/BPI_Bonus.BonusOnTarget` OtherActor false))
    (:`6`
      (message `/Game/Blueprints/Interfaces/BPI_Bonus.BonusRocket` OtherActor)))
  (`self.K2_DestroyActor`))

(fn `InitialSpeed`
  (set `self.Speed` (`KismetMathLibrary.RandomFloatInRange` 1500.0 2000.0))
  (set `MovementComponent.Velocity` (`KismetMathLibrary.MakeVector` (`self.Speed`)) (`self.ProjectileMovement`)))

(fn `SecondBallFunc`
  (params (Pawn :type "Actor Object Reference"))
  (message `/Game/Blueprints/Interfaces/BPI_Bonus.BonusSecondBall` Pawn))

(fn `SetColor`
  (`PrimitiveComponent.SetMaterial` (`self.Sphere`) 0 "/Game/Materials/MI_BonusBlue.MI_BonusBlue"))

(fn `UserConstructionScript`
  (`parent.UserConstructionScript`))
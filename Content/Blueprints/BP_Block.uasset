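; BP_Block is a destructible block that takes hits and can spawn a bonus when destroyed.
; Each hit lowers Health and swaps the cube for a Geometry Collection, unless the block is immortal.
; At minimum Health it enables physics, clears tags, asks its parent actor to spawn a bonus, then self-destructs after a random delay.
; It relays bonus events to the parent and handles timed immortality itself.
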(event `self.ReceiveBeginPlay`
  ;[0.02061 1 0.1526] BeginPlay
  (set `self.Health` 2))

(event `self.ReceiveHit`
  (params (MyComp :type "PrimitiveComponent Object Reference") (Other :type "Actor Object Reference") (OtherComp :type "PrimitiveComponent Object Reference") (bSelfMoved :type Boolean) (HitLocation :type "Vector Structure") (HitNormal :type "Vector Structure") (NormalImpulse :type "Vector Structure") (Hit :type "HitResult Structure (by ref)"))
  ;[1 0.9385 0] EventHit
  (if (`self.TakeDamage`)
    (`self.Death`)))

(event `Death`
  ;[1 0.164 0] DeathEvent
  (`/Engine/EditorBlueprintResources/StandardMacros.DoOnce` false
    (:`Completed`
      (`self.OnDeath`)
      (message `/Game/Blueprints/Interfaces/BPI_Bonus.SpawnBonus` (`self.GetParentActor`) (`self.K2_GetActorLocation`))
      (`KismetSystemLibrary.Delay` (`KismetMathLibrary.RandomFloatInRange` 0.4 1.0))
      (`self.K2_DestroyActor`))))

(event `self.ReceiveTick`
  (params (DeltaSeconds :type "Float (single-precision)")))

(event `/Game/Blueprints/Interfaces/BPI_Bonus.BonusBallSlowDown`
  (params (HasBonus :type Boolean))
  (message `/Game/Blueprints/Interfaces/BPI_Bonus.BonusBallSlowDown` (`self.GetParentActor`) HasBonus))

(event `/Game/Blueprints/Interfaces/BPI_Bonus.BonusBlocksImmortal`
  (set `self.IsImmortal` true)
  (message `/Game/Blueprints/Interfaces/BPI_Bonus.ApplyingBonus` (`self.GetParentActor`))
  (`KismetSystemLibrary.K2_SetTimerDelegate` (`|CreateDelegate` :!event `BonusImmortalEnds`) 5.0))

(event `/Game/Blueprints/Interfaces/BPI_Bonus.BonusOnTarget`
  (params (HasBonus :type Boolean))
  (message `/Game/Blueprints/Interfaces/BPI_Bonus.BonusOnTarget` (`self.GetParentActor`) HasBonus))

(fn `BonusImmortalEnds`
  (set `self.IsImmortal` false)
  (message `/Game/Blueprints/Interfaces/BPI_Bonus.BonusEnds` (`self.GetParentActor`)))

(fn `OnDeath`
  (bind _geometrycollection (`self.GeometryCollection`))
  (`PrimitiveComponent.SetSimulatePhysics` _geometrycollection true)
  (`PrimitiveComponent.SetCollisionObjectType` _geometrycollection "ECC_PhysicsBody")
  (`KismetArrayLibrary.Array_Clear` (`self.Tags`))
  (`PrimitiveComponent.SetCollisionObjectType` (`self.Box`) "ECC_PhysicsBody"))

(fn `OnTarget`
  (returns (HomeTarget :type "SceneComponent Object Reference"))
  (return (`self.DefaultSceneRoot`)))

(fn `TakeDamage`
  (returns (IsDeath :type Boolean))
  (bind _geometrycollection (`self.GeometryCollection`))
  (if (not (`self.IsImmortal`))
    (bind _result (`/Engine/EditorBlueprintResources/StandardMacros.DecrementInt` (`self.Health`))
      (:`  `
        (set `self.Health` (`KismetMathLibrary.Max` _result (`self.MinHealth`)))
        (`SceneComponent.SetHiddenInGame` (`self.Cube`) true false)
        (`SceneComponent.SetVisibility` _geometrycollection true false)
        (`SceneComponent.SetHiddenInGame` _geometrycollection false false)
        (return (<= (`self.Health`) (`self.MinHealth`)))))))

(fn `UserConstructionScript`
  (`SceneComponent.SetHiddenInGame` (`self.GeometryCollection`) true false)
  (`SceneComponent.SetHiddenInGame` (`self.Cube`) false false))
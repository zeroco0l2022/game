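; BP_Rocket is a short-lived projectile actor that flies straight along its forward direction.
; On BeginPlay it sets its ProjectileMovement velocity from the actor rotation and gives itself a brief lifespan.
; When it hits an actor tagged Block, it calls BonusRocketEnd and destroys itself.
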(event `self.ReceiveBeginPlay`
  (set `MovementComponent.Velocity` (* (`KismetMathLibrary.GetForwardVector` (`self.K2_GetActorRotation`)) 1000.0) (`self.ProjectileMovement`))
  (`self.SetLifeSpan` 0.5))

(event `self.ReceiveHit`
  (params (MyComp :type "PrimitiveComponent Object Reference") (Other :type "Actor Object Reference") (OtherComp :type "PrimitiveComponent Object Reference") (bSelfMoved :type Boolean) (HitLocation :type "Vector Structure") (HitNormal :type "Vector Structure") (NormalImpulse :type "Vector Structure") (Hit :type "HitResult Structure (by ref)"))
  (if (`self.ActorHasTag` Other "Block")
    (`self.BonusRocketEnd`)
    (`self.K2_DestroyActor`)))

(fn `UserConstructionScript`
  (`parent.UserConstructionScript`))
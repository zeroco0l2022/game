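; BP_Blocks is an actor that lays out a flat grid of child actors.
; Its construction script runs nested loops from zero through X and Y, adding a Child Actor Component at each step.
; Each component is offset on the X and Y axes by its loop index times Padding.
; The event graph holds only disabled placeholder events.
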(fn `UserConstructionScript`
  (for _index (range (+ (`self.X`) 1))
    (for _index_2 (range (+ (`self.Y`) 1))
      (`AddComponent|NODE_AddChildActorComponent-1` :`RelativeTransform` (`KismetMathLibrary.MakeTransform` (`KismetMathLibrary.MakeVector` (`KismetMathLibrary.Conv_IntToDouble` (* _index (`self.Padding`))) (`KismetMathLibrary.Conv_IntToDouble` (* _index_2 (`self.Padding`)))))))))
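; BP_Bonus is a moving bonus pickup that notifies whatever Pawn-tagged actor it hits, then destroys itself.
; On BeginPlay it launches along negative X at a random speed through its ProjectileMovement component.
; A looping timer re-fires ColorChange, which calls ColorFunc to re-arm the timer and flip the sphere between blue and red materials.
; The hit sends a BonusFunc message to the other actor, while this asset's own BonusFunc is empty.
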(event `self.ReceiveBeginPlay`
  ;[0.9267 0.3421 1] BeginPlay
  (`self.ColorChange`)
  (`self.InitialSpeed`))

(event `ColorChange`
  ;[0.2249 1 0.3694] ColorChanging
  (`self.ColorFunc` (delegate `ColorChange`)))

(event `self.ReceiveActorBeginOverlap`
  (params (OtherActor :type "Actor Object Reference"))
  (`parent.ReceiveActorBeginOverlap` OtherActor))

(event `self.ReceiveHit`
  (params (MyComp :type "PrimitiveComponent Object Reference") (Other :type "Actor Object Reference") (OtherComp :type "PrimitiveComponent Object Reference") (bSelfMoved :type Boolean) (HitLocation :type "Vector Structure") (HitNormal :type "Vector Structure") (NormalImpulse :type "Vector Structure") (Hit :type "HitResult Structure (by ref)"))
  (if (`self.ActorHasTag` Other "Pawn")
    (message `/Game/BPI_Bonus.BonusFunc` Other)
    (`self.K2_DestroyActor`)))

(fn `BonusFunc`)

(fn `ColorFunc`
  (params (Delegate :type Delegate))
  (bind _sphere (`self.Sphere`))
  (`KismetSystemLibrary.K2_SetTimerDelegate` Delegate 0.5 true)
  (`/Engine/EditorBlueprintResources/StandardMacros.FlipFlop`
    (:`A`
      (`PrimitiveComponent.SetMaterial` _sphere 0 "/Game/MI_BonusBlue.MI_BonusBlue"))
    (:`B`
      (`PrimitiveComponent.SetMaterial` _sphere 0 "/Game/MI_BonusRed.MI_BonusRed"))))

(fn `InitialSpeed`
  (set `self.Speed` (`KismetMathLibrary.RandomFloatInRange` 1000.0 1500.0))
  (set `MovementComponent.Velocity` (`KismetMathLibrary.MakeVector` (* (`self.Speed`) -1.0)) (`self.ProjectileMovement`)))

(fn `UserConstructionScript`
  (`parent.UserConstructionScript`))